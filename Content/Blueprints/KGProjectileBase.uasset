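; Base projectile Blueprint that damages KGCharacterBase characters other than its instigator.
; On overlapping such a character it applies direct damage, plays an impact sound and destroys itself.
; Its Destroyed event spawns an impulse particle effect and applies half damage in a small radius, so a direct hit also triggers the splash and any other destruction still does.
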(event `self.ReceiveActorBeginOverlap`
  (params (OtherActor :type "Actor Object Reference"))
  (bind _instigator (`self.Instigator`))
  (bind _askgcharacter_base (cast `/Game/Blueprints/KGCharacterBase` OtherActor))
  (if (not (== _askgcharacter_base _instigator))
    (`GameplayStatics.ApplyDamage` _askgcharacter_base (`self.ProjectileDamage`) (`Pawn.GetController` _instigator) self)
    (`GameplayStatics.PlaySoundAtLocation` "/Game/Assets/Sounds/ImpactCue.ImpactCue" (`self.K2_GetActorLocation`) (struct) 1.0 1.0 0.0 null null null)
    (`self.K2_DestroyActor`)))

(event `self.ReceiveDestroyed`
  (`GameplayStatics.SpawnEmitterAtLocation` "/Game/Assets/Effects/P_Impulse.P_Impulse" (`self.K2_GetActorLocation`))
  (`GameplayStatics.ApplyRadialDamage` :`BaseDamage` (/ (`self.ProjectileDamage`) 2.0) :`Origin` (`self.K2_GetActorLocation`) :`DamageRadius` 25.0 :`DamageCauser` self :`InstigatedByController` (`Pawn.GetController` (`self.Instigator`))))

(fn `UserConstructionScript`)