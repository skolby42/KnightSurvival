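; BaseSword is a melee weapon actor that damages nearby pawns when its TryDealDamage event is called.
; The event runs a sphere overlap at the sword mesh's location, ignoring the owner of the component the sword is attached to.
; Each pawn found takes HitDamage, and ImpactCue plays at that pawn's location.
; Tick, BeginPlay and the construction script are empty, so the hit check depends entirely on that event.
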(event `TryDealDamage`
  (bind _outactors (`KismetSystemLibrary.SphereOverlapActors` (`SceneComponent.K2_GetComponentLocation` (`self.SwordMesh`)) 70.0 (`|MakeArray` "ObjectTypeQuery3" :!type "EObjectTypeQuery Enum") null (`|MakeArray` (`ActorComponent.GetOwner` (`SceneComponent.GetAttachParent` (`self.DefaultSceneRoot`))))))
  (for _array_element _outactors
    (`GameplayStatics.ApplyDamage` _array_element (`self.HitDamage`))
    (`GameplayStatics.PlaySoundAtLocation` "/Game/Assets/Sounds/ImpactCue.ImpactCue" (`self.K2_GetActorLocation` _array_element) (struct) 1.0 1.0 0.0 null null null)))

(fn `UserConstructionScript`)