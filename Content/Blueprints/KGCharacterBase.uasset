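; Base knight character for player- and AI-controlled fighters, with melee, magic, health and death.
; Spawns a socketed sword, links the health bar widget and tints hair via a dynamic material.
; Montages drive combo attacks, magic and damage flinches, which are skipped during listed attack sections and block new attacks.
; Player death shows game over and ends the game; other knights are destroyed, while living knights play victory on game end.
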(event `self.ReceiveBeginPlay`
  (`self.CreateSword`)
  (`self.SetHealthBarOwningKnight`)
  (bind _askggame_mode (cast `/Game/Blueprints/KGGameMode` (`GameplayStatics.GetGameMode`)))
  (add `/Game/Blueprints/KGGameMode.EndGameDispatch` _askggame_mode (delegate `EndGameDance`)))

(event `EndGameDance`
  (if (> (`self.Health`) 0.0)
    (`CharacterMovementComponent.DisableMovement` (`self.CharacterMovement`))
    (`self.PlayAnimMontage` "/Game/Assets/Knight/Victory_Montage.Victory_Montage")))

(event `TryMelee`
  (bind _returnvalue (`SkeletalMeshComponent.GetAnimInstance` (`self.Mesh`)))
  (bind _returnvalue_2 (`AnimInstance.Montage_GetCurrentSection` _returnvalue "/Game/Assets/Knight/KnightAttack.KnightAttack"))
  (if (and (> (`self.Health`) 0.0) (not (`self.IsFlinching`)))
    (if (`AnimInstance.Montage_IsActive` _returnvalue "/Game/Assets/Knight/KnightAttack.KnightAttack")
      (switch `name` _returnvalue_2
        (:`Attack1`
          (`AnimInstance.Montage_SetNextSection` _returnvalue _returnvalue_2 "Attack2" null)))
      (else
        (`self.PlayAnimMontage` "/Game/Assets/Knight/KnightAttack.KnightAttack" 1.0 "Attack1")))))

(event `TryMagic`
  (if (and (> (`self.Health`) 0.0) (not (`self.IsFlinching`)))
    (`self.PlayAnimMontage` "/Game/Assets/Knight/MagicShootMontage.MagicShootMontage")))

(event `LaunchMagicProjectile`
  (`GameplayStatics.PlaySoundAtLocation` "/Game/Assets/Sounds/FireCue.FireCue" (`self.K2_GetActorLocation`) (struct) 1.0 1.0 0.0 null null null)
  (`|SpawnActorFromClass` "/Game/Blueprints/KGProjectileBase.KGProjectileBase_C" (`SceneComponent.K2_GetComponentToWorld` (`self.Arrow1`)) "Undefined" "OverrideRootScale" null self))

(event `UsePrimaryAttack`
  (`self.TryMelee`))

(event `CreateSword`
  (bind _returnvalue (`|SpawnActorFromClass` "/Game/Blueprints/BaseSword.BaseSword_C" (`self.GetTransform`) "Undefined" "OverrideRootScale" null null))
  (`self.K2_AttachToComponent` _returnvalue (`self.Mesh`) "Sword" "SnapToTarget" "SnapToTarget" "SnapToTarget" false)
  (set `self.Weapon` _returnvalue))

(event `SetHealthBarOwningKnight`
  (bind _ashealth_bar_widget (cast `/Game/Blueprints/HealthBarWidget` (`WidgetComponent.GetUserWidgetObject` (`self.HealthBar`))))
  (`/Game/Blueprints/HealthBarWidget.SetOwningKnightCharacter` _ashealth_bar_widget self))

(event `self.ReceiveAnyDamage`
  (params (Damage :type "Float (single-precision)") (DamageType :type "DamageType Object Reference") (InstigatedBy :type "Controller Object Reference") (DamageCauser :type "Actor Object Reference"))
  (bind _returnvalue (`SkeletalMeshComponent.GetAnimInstance` (`self.Mesh`)))
  (bind _output_get (set `self.Health` (- (`self.Health`) Damage)))
  (if (<= _output_get 0.0)
    (`/Engine/EditorBlueprintResources/StandardMacros.DoOnce` false
      (:`Completed`
        (set `self.IsFlinching` true)
        (`self.CharacterDeath`)))
    (else
      (set `self.IsFlinching` true)
      (if (`AnimInstance.Montage_IsActive` _returnvalue "/Game/Assets/Knight/KnightAttack.KnightAttack")
        (if (`KismetArrayLibrary.Array_Contains` (`self.AttackMoves`) (`AnimInstance.Montage_GetCurrentSection` _returnvalue "/Game/Assets/Knight/KnightAttack.KnightAttack"))
          (set `self.IsFlinching` false)
          (else
            (bind _returnvalue_2 (`self.PlayAnimMontage` "/Game/Assets/Knight/PlayerFlinch.PlayerFlinch" 1.0 "FlinchBig"))
            (`KismetSystemLibrary.Delay` _returnvalue_2)
            (set `self.IsFlinching` false)))
        (else
          (bind _returnvalue_3 (`self.PlayAnimMontage` "/Game/Assets/Knight/PlayerFlinch.PlayerFlinch" 1.0 "FlinchSmall"))
          (`KismetSystemLibrary.Delay` _returnvalue_3)
          (set `self.IsFlinching` false))))))

(event `CharacterDeath`
  (bind _weapon (`self.Weapon`))
  (bind _hud_widget (`/Game/Blueprints/KGPlayerControllerBase.HUD_Widget` (cast `/Game/Blueprints/KGPlayerControllerBase` (`self.GetController`) :!pure true)))
  (bind _returnvalue (`self.PlayAnimMontage` "/Game/Assets/Knight/PlayerDeath.PlayerDeath"))
  (`CharacterMovementComponent.DisableMovement` (`self.CharacterMovement`))
  (if (`Controller.IsPlayerController` (`self.GetController`))
    (`UserWidget.PlayAnimation` _hud_widget (`/Game/Blueprints/KG_HUD.GameOverPopupAnim` _hud_widget) 0.0 1 "Forward" 1.0 false)
    (`self.SetActorHiddenInGame` false)
    (`/Game/Blueprints/KGGameMode.EndGame` (cast `/Game/Blueprints/KGGameMode` (`GameplayStatics.GetGameMode`) :!pure true))
    (else
      (`KismetSystemLibrary.Delay` _returnvalue)
      (`self.K2_DestroyActor`)
      (`/Engine/EditorBlueprintResources/StandardMacros.IsValid` _weapon
        (:`Is Valid`
          (`self.K2_DestroyActor` _weapon))))))

(fn `UserConstructionScript`
  (bind _returnvalue (`PrimitiveComponent.CreateDynamicMaterialInstance` (`self.Mesh`) 0 null "None"))
  (`MaterialInstanceDynamic.SetVectorParameterValue` _returnvalue "HairColor" (`self.HairColor`)))