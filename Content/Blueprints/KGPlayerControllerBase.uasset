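; Base player controller that drives a top-down KG character with cursor aiming, camera-relative movement, jump, and melee and magic attacks.
; On BeginPlay it creates the HUD and binds to KGGameMode dispatchers to play wave and game-won popup animations.
; Each tick it traces under the cursor to yaw a living pawn toward the hit point.
; A DoProcessMouse flag gates aiming and attacks, while the menu key calls the game mode.
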(event `self.ReceiveBeginPlay`
  (set `self.bShowMouseCursor` true)
  (bind _returnvalue (`|CreateWidget` "/Game/Blueprints/KG_HUD.KG_HUD_C"))
  (bind _output_get (set `self.HUD_Widget` _returnvalue))
  (`UserWidget.AddToViewport` _output_get 0)
  (bind _askggame_mode (cast `/Game/Blueprints/KGGameMode` (`GameplayStatics.GetGameMode`)))
  (add `/Game/Blueprints/KGGameMode.NewWaveDispatch` _askggame_mode (delegate `ShowWavePopup`))
  (add `/Game/Blueprints/KGGameMode.GameWonDispatch` _askggame_mode (delegate `ShowGameWonPopup`)))

(event `ShowWavePopup`
  (bind _hud_widget (`self.HUD_Widget`))
  (bind _askggame_mode (cast `/Game/Blueprints/KGGameMode` (`GameplayStatics.GetGameMode`)))
  (set `/Game/Blueprints/KG_HUD.Wave` (`/Game/Blueprints/KGGameMode.WaveIndex` _askggame_mode) _hud_widget)
  (`UserWidget.PlayAnimation` _hud_widget (`/Game/Blueprints/KG_HUD.WaveCompletedPopupAnim` _hud_widget) 0.0 1 "Forward" 1.0 false))

(event `ShowGameWonPopup`
  (bind _hud_widget (`self.HUD_Widget`))
  (`UserWidget.PlayAnimation` _hud_widget (`/Game/Blueprints/KG_HUD.GameWonPopupAnim` _hud_widget) 0.0 1 "Forward" 1.0 false))

(event `self.ReceiveTick`
  (params (DeltaSeconds :type "Float (single-precision)"))
  (`self.ProcessMouse`))

(event `ProcessMouse`
  (bind (_hitresult _returnvalue) (`self.GetHitResultUnderCursorByChannel` "TraceTypeQuery1"))
  (bind _returnvalue_2 (`self.K2_GetPawn`))
  (bind _returnvalue_3 (`self.K2_GetPawn`))
  (bind (_returnvalue_roll _returnvalue_pitch _returnvalue_yaw) (`KismetMathLibrary.BreakRotator` (`KismetMathLibrary.Conv_VectorToRotator` (`KismetMathLibrary.GetDirectionUnitVector` (`self.K2_GetActorLocation` _returnvalue_2) (`.Location` (`GameplayStatics.BreakHitResult` _hitresult))))))
  (if (`self.DoProcessMouse`)
    (`/Engine/EditorBlueprintResources/StandardMacros.IsValid` _returnvalue_3
      (:`Is Valid`
        (bind _askgcharacter_base (cast `/Game/Blueprints/KGCharacterBase` _returnvalue_3))
        (if (and (> (`/Game/Blueprints/KGCharacterBase.Health` _askgcharacter_base) 0.0) _returnvalue)
          (`self.K2_SetActorRotation` _returnvalue_2 (`KismetMathLibrary.MakeRotator` 0.0 0.0 _returnvalue_yaw) false))))))

(event `InputAxis|Up`
  (params (AxisValue :type "Float (single-precision)"))
  (bind _returnvalue (`self.K2_GetPawn`))
  (`/Engine/EditorBlueprintResources/StandardMacros.IsValid` _returnvalue
    (:`Is Valid`
      (`Pawn.AddMovementInput` _returnvalue (`self.GetActorUpVector` (`self.PlayerCameraManager`)) AxisValue false))))

(event `InputAxis|Right`
  (params (AxisValue :type "Float (single-precision)"))
  (bind _returnvalue (`self.K2_GetPawn`))
  (`/Engine/EditorBlueprintResources/StandardMacros.IsValid` _returnvalue
    (:`Is Valid`
      (`Pawn.AddMovementInput` _returnvalue (`self.GetActorRightVector` (`self.PlayerCameraManager`)) AxisValue false))))

(event `InputAction|Jump`
  (params (Key :type "Key Structure"))
  (bind _returnvalue (`self.K2_GetPawn`))
  (:`Pressed`
    (`/Engine/EditorBlueprintResources/StandardMacros.IsValid` _returnvalue
      (:`Is Valid`
        (bind _ascharacter (cast `Character` _returnvalue))
        (`Character.Jump` _ascharacter)))))

(event `InputAction|MeleeAttack`
  (params (Key :type "Key Structure"))
  (bind _returnvalue (`self.K2_GetPawn`))
  (:`Pressed`
    (if (`self.DoProcessMouse`)
      (`/Engine/EditorBlueprintResources/StandardMacros.IsValid` _returnvalue
        (:`Is Valid`
          (bind _askgcharacter_base (cast `/Game/Blueprints/KGCharacterBase` _returnvalue))
          (`/Game/Blueprints/KGCharacterBase.TryMelee` _askgcharacter_base))))))

(event `InputAction|MagicAttack`
  (params (Key :type "Key Structure"))
  (bind _returnvalue (`self.K2_GetPawn`))
  (:`Pressed`
    (if (`self.DoProcessMouse`)
      (`/Engine/EditorBlueprintResources/StandardMacros.IsValid` _returnvalue
        (:`Is Valid`
          (bind _askgcharacter_base (cast `/Game/Blueprints/KGCharacterBase` _returnvalue))
          (`/Game/Blueprints/KGCharacterBase.TryMagic` _askgcharacter_base))))))

(event `InputAction|MainMenu`
  (params (Key :type "Key Structure"))
  (:`Pressed`
    (bind _askggame_mode (cast `/Game/Blueprints/KGGameMode` (`GameplayStatics.GetGameMode`)))
    (`/Game/Blueprints/KGGameMode.ShowMainMenu` _askggame_mode)))

(fn `UserConstructionScript`)